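; Snake pawn for single or two-player play that eats food to grow, score and advance levels.
; At startup it reads game settings and spawns the first level; player one also finds the second snake and forwards keyboard direction to it.
; Food overlaps add tail and score with rising pickup pitch, completing the level past the size requirement.
; Other overlaps after brief invincibility kill it, save score or multiplayer winner, and load LoseMap.
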(event EventBeginPlay
  (Utilities|FlowControl|DelayUntilNextTick)
  (if (Variables|Default|GetisPlayerOne)
    (bind _outactors (Actor|GetAllActorsOfClass "BP_Snake_C"))
    (for _array_element _outactors
      (if (not (== _array_element self))
        (Variables|Default|SetP2 _array_element)
        (Variables|Default|SetcurrentLevel 1)
        (Variables|Default|SetScore 0)
        (bind _returnvalue (Actor|GetActorOfClass "/Game/BP_LevelSpawner.BP_LevelSpawner_C"))
        (Default|SpawnLevel _returnvalue)
        (bind _ascustom_game_instance (Utilities|Casting|CastToCustomGameInstance (Game|GetGameInstance)))
        (Variables|Default|SetstartSize (Variables|/Game/CustomGameInstance.CustomGameInstance_C|GetStartSize _ascustom_game_instance))
        (Variables|Default|SetfoodRequirement (Variables|/Game/CustomGameInstance.CustomGameInstance_C|GetScoreRequirement _ascustom_game_instance))
        (Variables|Default|SetIsMultiplayer (Variables|/Game/CustomGameInstance.CustomGameInstance_C|GetMultiplayer _ascustom_game_instance))))
    (else
      (Variables|Default|SetcurrentLevel 1)
      (Variables|Default|SetScore 0)
      (bind _returnvalue_2 (Actor|GetActorOfClass "/Game/BP_LevelSpawner.BP_LevelSpawner_C"))
      (Default|SpawnLevel _returnvalue_2)
      (bind _ascustom_game_instance_2 (Utilities|Casting|CastToCustomGameInstance (Game|GetGameInstance)))
      (Variables|Default|SetstartSize (Variables|/Game/CustomGameInstance.CustomGameInstance_C|GetStartSize _ascustom_game_instance_2))
      (Variables|Default|SetfoodRequirement (Variables|/Game/CustomGameInstance.CustomGameInstance_C|GetScoreRequirement _ascustom_game_instance_2))
      (Variables|Default|SetIsMultiplayer (Variables|/Game/CustomGameInstance.CustomGameInstance_C|GetMultiplayer _ascustom_game_instance_2)))))

(event Collision|EventActorBeginOverlap
  (params (OtherActor :type Actor%20Object%20Reference))
  (if (Variables|Default|GetisAlive)
    (bind _asbp_food (Utilities|Casting|CastToBP_Food OtherActor)
      (:then
        (CallFunction|CollectFood _asbp_food)
        (if (< (Variables|Default|GetfoodRequirement) (Variables|Default|Getsize))
          (CallFunction|CompleteLevel)))
      (:CastFailed
        (if (< (Variables|Default|GetstartingInvic) (Actor|GetGameTimeSinceCreation))
          (Variables|Default|SetisAlive false)
          (Actor|Tick|SetActorTickEnabled false)
          (Collision|SetCollisionEnabled (Variables|Default|GetColSphere) "NoCollision")
          (if (Variables|Default|GetIsMultiplayer)
            (bind _ascustom_game_instance (Utilities|Casting|CastToCustomGameInstance (Game|GetGameInstance)))
            (Variables|/Game/CustomGameInstance.CustomGameInstance_C|SetWinner _ascustom_game_instance (Utilities|String|Append (select (Variables|Default|GetisPlayerOne) "PLAYER 2" "PLAYER 1") " WINS!")))
          (Class|LevelStreamingDynamic|LoadLevelInstance "LoseMap" "0, 0, 0" "0, 0, 0" "" 0 false)
          (CallFunction|SetScoreinGameState)
          (CallFunction|PlaySound "/Game/Audio/hurt_Cue.hurt_Cue"))))))

(event EventPossessed
  (params (NewController :type Controller%20Object%20Reference))
  (Utilities|Casting|CastToPlayerController NewController)
  (bind _output_get (Variables|Default|SetpController (Class|GameplayStatics|GetPlayerControllerfromID)))
  (Input|EnableInput _output_get))

(event EventTick
  (params (DeltaSeconds :type Float%20%28single-precision%29))
  (if (and (Variables|Default|GetisPlayerOne) (Utilities|IsValid (Variables|Default|GetP2)))
    (bind _output_get (Variables|Default|SetkeyboardDirection (Math|Conversions|ToVector2D(Vector) (Math|Vector|MakeVector (Input|AxisValues|GetVertical) (Input|AxisValues|GetHorizontal) 0.0))))
    (Variables|/Script/Snuk.SnakeBase|SetkeyboardDirection (Variables|Default|GetP2) _output_get)))

(fn ConstructionScript)

(fn SetScoreinGameState
  (bind _ascustom_game_instance (Utilities|Casting|CastToCustomGameInstance (Game|GetGameInstance)))
  (bind _output_get (Variables|/Game/CustomGameInstance.CustomGameInstance_C|SetScore _ascustom_game_instance (Variables|Default|GetScore)))
  (if (< (Variables|/Game/CustomGameInstance.CustomGameInstance_C|GetHighScore _ascustom_game_instance) _output_get)
    (Variables|/Game/CustomGameInstance.CustomGameInstance_C|SetHighScore _ascustom_game_instance _output_get)))

(fn CompleteLevel
  (Class|SnakeBase|NextLevel)
  (bind _foundwidgets (Widget|GetAllWidgetsOfClass "/Game/UI/GameUI.GameUI_C" true))
  (Default|LevelUp (Utilities|Array|Get(acopy) _foundwidgets))
  (bind _returnvalue (Actor|GetActorOfClass "/Game/BP_LevelSpawner.BP_LevelSpawner_C"))
  (Default|SpawnLevel _returnvalue (Variables|Default|GetcurrentLevel))
  (CallFunction|PlaySound "/Game/Audio/nextlevel_Cue.nextlevel_Cue"))

(fn CollectFood
  (params (Food :type BP%20Food%20Object%20Reference))
  (Default|Collected Food)
  (Class|Food|SpawnFood Food)
  (Class|SnakeBase|SpawnTail)
  (Variables|Default|SetScore (+ (* 50 (Variables|Default|GetcurrentLevel)) (Variables|Default|GetScore)))
  (CallFunction|SetScoreinGameState)
  (bind _returnvalue (Audio|CreateSound2D "/Game/Audio/pickupfood_Cue.pickupfood_Cue" 1.0 1.0 0.0 0))
  (Audio|Parameter|SetFloatParameter _returnvalue "CollectablePitch" (/ (Math|Conversions|ToFloat(Integer) (Variables|Default|Getsize)) (Math|Conversions|ToFloat(Integer) (Variables|Default|GetfoodRequirement))) :!class /Script/AudioExtensions.AudioParameterControllerInterface)
  (Audio|Components|Audio|Play _returnvalue 0.0))

(fn PlaySound
  (params (Sound :type Sound%20Cue%20Object%20Reference))
  (Audio|PlaySound2D Sound 1.0 1.0 0.0 0 0))
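; Level spawner actor that replaces the current wall layout with the level for a given index.
; On BeginPlay and on each SpawnLevel call, it sets Area from the custom game instance's AreaSize, scaled down by a constant.
; SpawnLevel then destroys every Wall actor in the world and passes the index to CreateLevel, whose logic is defined outside these graphs.
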(event EventBeginPlay
  (bind _ascustom_game_instance (Utilities|Casting|CastToCustomGameInstance (Game|GetGameInstance)))
  (Variables|Default|Setarea (/ (Variables|/Game/CustomGameInstance.CustomGameInstance_C|GetAreaSize _ascustom_game_instance) 1e+03)))

(event Collision|EventActorBeginOverlap
  (params (OtherActor :type Actor%20Object%20Reference)))

(event EventTick
  (params (DeltaSeconds :type Float%20%28single-precision%29)))

(fn ConstructionScript)

(fn SpawnLevel
  (params (Index :type Integer))
  (bind _ascustom_game_instance (Utilities|Casting|CastToCustomGameInstance (Game|GetGameInstance)))
  (Variables|Default|Setarea (/ (Variables|/Game/CustomGameInstance.CustomGameInstance_C|GetAreaSize _ascustom_game_instance) 1e+03))
  (bind _outactors (Actor|GetAllActorsOfClass "/Game/Wall.Wall_C"))
  (for _array_element _outactors
    (Actor|DestroyActor _array_element))
  (Class|LevelSpawner|CreateLevel Index))